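; BP_Plane is a plane that flies forward continuously and responds to a Turn input axis.
; Each tick it offsets its location along the actor's forward vector by MoveSpeed scaled by delta time, without sweeping for collision.
; Non-zero Turn input adds world-space roll to the Body component, scaled by RotateSpeed and delta time, with no pitch or yaw.
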(event EventTick
  (params (DeltaSeconds :type Float%20%28single-precision%29))
  (Transformation|SetActorLocation (+ (Transformation|GetActorLocation) (* (* DeltaSeconds (Variables|Default|GetMoveSpeed)) (Transformation|GetActorForwardVector))) false false))

(event Input|AxisEvents|InputAxisTurn
  (params (AxisValue :type Float%20%28single-precision%29))
  (if (!= AxisValue 0.0)
    (Transformation|AddWorldRotation (Variables|Default|GetBody) (Math|Rotator|MakeRotator (* AxisValue (* (stale EventTick DeltaSeconds) (Variables|Default|GetRotateSpeed))) 0.0 0.0) false false)))

(fn ConstructionScript)